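; SpeedZone is a boost zone that launches a PhysicsBallBP along the forward direction of its Cube.
; On overlap it zeroes the ball's linear velocity, prints a debug "hit", then applies a velocity-change impulse scaled by Speed, so incoming velocity and mass don't affect the launch.
; The construction script runs a line trace only for its debug drawing, previewing the launch direction with length equal to Speed.
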(event Collision|EventActorBeginOverlap
  (params (OtherActor :type Actor%20Object%20Reference))
  (bind _asphysics_ball_bp (Utilities|Casting|CastToPhysicsBallBP OtherActor))
  (Physics|SetPhysicsLinearVelocity (Variables|/Game/RollingBP/Blueprints/PhysicsBallBP.PhysicsBallBP_C|GetBall _asphysics_ball_bp) "0, 0, 0" false "None")
  (Development|PrintString "hit")
  (Physics|AddImpulse (Variables|/Game/RollingBP/Blueprints/PhysicsBallBP.PhysicsBallBP_C|GetBall _asphysics_ball_bp) (* (Math|Vector|GetForwardVector (Variables|Default|GetCube)) (Variables|Default|GetSpeed)) "None" true))

(fn ConstructionScript
  (bind _cube (Variables|Default|GetCube))
  (bind _returnvalue (Transformation|GetWorldLocation _cube))
  (Class|KismetSystemLibrary|LineTraceMultiforObjects _returnvalue (+ _returnvalue (* (Math|Vector|GetForwardVector _cube) (Variables|Default|GetSpeed))) (LocalVariables|GetNewLocalVar_0) false 0 "ForDuration" true))