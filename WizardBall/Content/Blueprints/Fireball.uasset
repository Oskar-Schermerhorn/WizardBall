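; Fireball actor that knocks players' physics balls upward and removes ice ramps on overlap.
; Its sphere's world scale sets both its lifetime and the strength of the launch.
; A hit on a non-owner PhysicsBallBP stops and interrupts the ball, applies a vertical impulse, then destroys the fireball.
; It passes through its owner and destroyed IceRamps, while any other overlap destroys it.
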(event Collision|EventActorBeginOverlap
  (params (OtherActor :type Actor%20Object%20Reference))
  ;[1 1 1] handle fireball hitting something
  (bind _asphysics_ball_bp (Utilities|Casting|CastToPhysicsBallBP OtherActor)
    (:then
      (if (!= OtherActor (Components|GetOwner))
        (Development|PrintString "player")
        (Physics|SetPhysicsLinearVelocity (Variables|/Game/RollingBP/Blueprints/PhysicsBallBP.PhysicsBallBP_C|GetBall _asphysics_ball_bp) "0, 0, 0" false "None")
        (Class|PrimitiveComponent|SetPhysicsAngularVelocityinDegrees (Variables|/Game/RollingBP/Blueprints/PhysicsBallBP.PhysicsBallBP_C|GetBall _asphysics_ball_bp) "0, 0, 0" false "None")
        (Default|Interrupt _asphysics_ball_bp)
        (Physics|AddImpulse (Variables|/Game/RollingBP/Blueprints/PhysicsBallBP.PhysicsBallBP_C|GetBall _asphysics_ball_bp) (Math|Vector|MakeVector 0.0 0.0 (+ (* (Math|Vector|VectorLength (Transformation|GetWorldScale (Variables|Default|GetSphere))) 1e+02) 1e+03)) "None" true)
        (Actor|DestroyActor)))
    (:CastFailed
      (bind _asice_ramp (Utilities|Casting|CastToIceRamp OtherActor)
        (:then
          (Development|PrintString "ice")
          (Actor|DestroyActor _asice_ramp))
        (:CastFailed
          (Actor|DestroyActor)
          (Development|PrintString (Utilities|String|Append "destroyed by " (Utilities|GetDisplayName OtherActor))))))))

(event EventBeginPlay
  (bind _sphere (Variables|Default|GetSphere))
  (bind _returnvalue (Transformation|GetWorldScale _sphere))
  (bind _returnvalue_2 (Math|Vector|VectorLength _returnvalue))
  (Utilities|FlowControl|Delay 0.2)
  (Utilities|IsValid _sphere
    (:Is%20Valid
      (Development|PrintString (Utilities|String|ToString(Float) _returnvalue_2))
      (Utilities|FlowControl|Delay _returnvalue_2)
      (Actor|DestroyActor)
      (Development|PrintString "destroy"))))

(fn ConstructionScript)