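; Placement preview actor for an ice ramp spell that shows where the ramp would go and whether that spot is valid.
; Each tick it line-traces along the supplied camera's forward vector from a raised start point, moves to the hit and yaws toward the camera.
; Near-flat surfaces set Valid, and a dynamic material recolors the cube as valid or invalid, or with an invisible color over KillZ volumes.
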(event Custom|setCamera
  (params (NewParam :type Object%20Object%20Reference) (CastRange :type Float%20%28single-precision%29) (ObjectTypes :type Array%20of%20EObjectTypeQuery%20Enums :default "ObjectTypeQuery1"))
  ;[1 1 1] set camera so it can update location
  (Variables|Default|SetCamera NewParam)
  (Variables|Default|SetCastRange CastRange)
  (Variables|Default|SetObject%20Types ObjectTypes))

(event EventTick
  (params (DeltaSeconds :type Float%20%28single-precision%29))
  (bind _material (Variables|Default|GetMaterial))
  ;[1 1 1] moving the preview
  (if (Utilities|IsValid (Variables|Default|GetCamera))
    (bind _ascamera_component (Utilities|Casting|CastToCameraComponent (Variables|Default|GetCamera)))
    (bind _outhit (Collision|LineTraceForObjects (Math|Vector|MakeVector (.x (Transformation|GetWorldLocation _ascamera_component)) (.y (Transformation|GetWorldLocation _ascamera_component)) (+ (.z (Transformation|GetWorldLocation _ascamera_component)) 5e+02)) (+ (Math|Vector|MakeVector (.x (Transformation|GetWorldLocation _ascamera_component)) (.y (Transformation|GetWorldLocation _ascamera_component)) (+ (.z (Transformation|GetWorldLocation _ascamera_component)) 5e+02)) (* (Math|Vector|GetForwardVector _ascamera_component) (Variables|Default|GetCastRange))) (Variables|Default|GetObject%20Types) false 0 "None"))
    (Utilities|Casting|CastToKillZVolume (.hitactor _outhit)
      (:then
        (Variables|Default|SetVisible false))
      (:CastFailed
        (Variables|Default|SetVisible true)))
    (Transformation|SetWorldLocation (Variables|Default|GetDefaultSceneRoot) (.location _outhit) false true)
    ;[1 1 1] update rotation so it faces player
    (bind _ascamera_component_2 (Utilities|Casting|CastToCameraComponent (Variables|Default|GetCamera)))
    (Transformation|SetWorldRotation (Variables|Default|GetDefaultSceneRoot) (Math|Rotator|MakeRotator 0.0 0.0 (+ (.yaw (Transformation|GetWorldRotation _ascamera_component_2)) 1.8e+02)) false false)
    ;[1 1 1] change color if it is valid
    (Variables|Default|SetValid (Math|Float|NearlyEqual(Float) (.z (.normal _outhit)) 1.0 0.1))
    (if (Variables|Default|GetVisible)
      (if (Math|Float|NearlyEqual(Float) (.z (.normal _outhit)) 1.0 0.1)
        (Rendering|Material|SetVectorParameterValue _material "Base Color" (Math|Conversions|ToLinearColor(Color) (Variables|Default|GetValidColor)) :!class /Script/Engine.MaterialInstanceDynamic)
        (Rendering|Material|SetMaterial (Variables|Default|GetCube1) 0 _material)
        (else
          (Rendering|Material|SetVectorParameterValue _material "Base Color" (Math|Conversions|ToLinearColor(Color) (Variables|Default|GetInvalidColor)) :!class /Script/Engine.MaterialInstanceDynamic)
          (Rendering|Material|SetMaterial (Variables|Default|GetCube1) 0 _material)))
      (else
        (Rendering|Material|SetVectorParameterValue _material "Base Color" (Math|Conversions|ToLinearColor(Color) (Variables|Default|GetInvisibleColor)) :!class /Script/Engine.MaterialInstanceDynamic)
        (Rendering|Material|SetMaterial (Variables|Default|GetCube1) 0 _material)))))

(event EventBeginPlay
  ;[1 1 1] create dynamic material to be edited later
  (bind _returnvalue (Rendering|Material|CreateDynamicMaterialInstance "/Game/RollingBP/Blueprints/SpellMaterial.SpellMaterial" "" "None" :!class /Script/Engine.KismetMaterialLibrary))
  (bind _output_get (Variables|Default|SetMaterial _returnvalue))
  (Rendering|Material|SetVectorParameterValue _output_get "Base Color" (Math|Conversions|ToLinearColor(Color) (Variables|Default|GetValidColor)) :!class /Script/Engine.MaterialInstanceDynamic)
  (Rendering|Material|SetMaterial (Variables|Default|GetCube1) 0 _output_get))

(fn ConstructionScript)