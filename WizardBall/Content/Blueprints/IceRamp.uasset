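; IceRamp is an actor whose Cube1 component rises into place from below, apparently as a spawned ice ramp.
; The construction script saves Cube1's location as CreationLocation, teleports the actor 320 units down, then records StartLocation, which the file never reads.
; Each Tick moves Cube1 a tenth of the remaining distance toward CreationLocation, giving a frame-rate-dependent ease-out without sweeping.
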(event EventTick
  (params (DeltaSeconds :type Float%20%28single-precision%29))
  (Transformation|SetWorldLocation (Variables|Default|GetCube1) (Math|Vector|Lerp(Vector) (Transformation|GetWorldLocation (Variables|Default|GetCube1)) (Variables|Default|GetCreationLocation) 0.1) false false))

(fn ConstructionScript
  (bind _cube1 (Variables|Default|GetCube1))
  (bind _returnvalue (Transformation|GetWorldLocation _cube1))
  (Variables|Default|SetCreationLocation (Math|Vector|MakeVector (.x _returnvalue) (.y _returnvalue) (.z _returnvalue)))
  (Transformation|Teleport (Math|Vector|MakeVector (.x _returnvalue) (.y _returnvalue) (- (.z _returnvalue) 3.2e+02)) "0, 0, 0")
  (Variables|Default|SetStartLocation (Transformation|GetWorldLocation (Variables|Default|GetCube1))))